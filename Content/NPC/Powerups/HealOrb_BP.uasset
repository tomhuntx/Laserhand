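; HealOrb_BP is a shootable heal powerup pawn that rewards the player with healing when killed.
; On Tick, one-shot flags start its sound and spawn its default controller.
; OnDamage and OnDeath play effects and trigger PlayerUI score animations, with death also calling the player's OnKill and OnKillHeal and stopping the sound.
; After a timed delay from BeginPlay, it stops the sound and destroys itself if that sound is still valid.
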(event EventOnDeath
  (bind _sounds (Variables|Default|GetSounds))
  (Audio|SpawnSoundatLocation "/Game/FirstPerson/Audio/PowerupDestroy.PowerupDestroy" (Transformation|GetWorldLocation (Variables|Default|GetCapsuleComponent)) "0, 0, 0" 1.0 1.0 0.0 0 0)
  (Game|SpawnActorfromClass "/Game/NPC/Powerups/HealDestroyFX.HealDestroyFX_C" (Transformation|GetWorldTransform (Variables|Default|GetCapsuleComponent)) "Undefined" 0 0)
  (bind _asfirst_person_character (Utilities|Casting|CastToFirstPersonCharacter (Game|GetPlayerCharacter 0)))
  (Default|OnKill _asfirst_person_character)
  (Default|OnKillHeal _asfirst_person_character)
  (bind _foundwidgets (Widget|GetAllWidgetsOfClass "/Game/UI/PlayerUI.PlayerUI_C" false))
  (Default|ScoreAnim _foundwidgets 2)
  (Utilities|IsValid _sounds
    (:Is%20Valid
      (Audio|Components|Audio|Stop _sounds))))

(event EventOnDamage
  (params (ProjTransform :type Transform))
  (Audio|SpawnSoundatLocation "/Game/FirstPerson/Audio/HitEnemyLogCue.HitEnemyLogCue" (Transformation|GetWorldLocation (Variables|Default|GetCapsuleComponent)) "0, 0, 0" 1.0 1.0 0.0 0 0)
  (Game|SpawnActorfromClass "/Game/NPC/Enemy/EnemySparks.EnemySparks_C" ProjTransform "Undefined" 0 0)
  (bind _foundwidgets (Widget|GetAllWidgetsOfClass "/Game/UI/PlayerUI.PlayerUI_C" false))
  (Default|ScoreAnim _foundwidgets))

(event EventTick
  (params (DeltaSeconds :type Float%20%28single-precision%29))
  (if (Variables|Default|GetPlayAudio)
    (bind _returnvalue (Audio|SpawnSoundatLocation "/Game/FirstPerson/Audio/PowerupLogCue.PowerupLogCue" (Transformation|GetWorldLocation (Variables|Default|GetCapsuleComponent)) "0, 0, 0" 1e+02 1.0 0.0 0 0))
    (Variables|Default|SetSounds _returnvalue)
    (Variables|Default|SetPlayAudio false))
  (if (Variables|Default|GetSpawnOwnAI)
    (Pawn|SpawnDefaultController)
    (Variables|Default|SetSpawnOwnAI false)))

(event EventBeginPlay
  (bind _sounds (Variables|Default|GetSounds))
  (Utilities|FlowControl|Delay 23.0)
  (Utilities|IsValid _sounds
    (:Is%20Valid
      (Audio|Components|Audio|Stop _sounds)
      (Actor|DestroyActor))))

(fn ConstructionScript)