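; Flying enemy that fires lasers when the player is within range and reports hits and kills to the player's UI.
; Tick optionally spawns its AI controller, spins a part faster as the randomized fire timer builds, and flags whether it is on-screen via screen projection.
; While in range, a stop flag eases fly speed to zero.
; Damage and death events spawn effects and sounds, with death also notifying the player character.
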(event EventOnDeath
  (Audio|SpawnSoundatLocation "/Game/StarterContent/Audio/Explosion_Cue.Explosion_Cue" (Transformation|GetWorldLocation (Variables|Default|GetCapsuleComponent)) "0, 0, 0" 1.0 1.0 0.0 0 0)
  (Game|SpawnActorfromClass "/Game/NPC/Enemy/EnemyExplosion.EnemyExplosion_C" (Transformation|GetWorldTransform (Variables|Default|GetCapsuleComponent)) "Undefined" 0 0)
  (bind _asfirst_person_character (Utilities|Casting|CastToFirstPersonCharacter (Game|GetPlayerCharacter 0)))
  (Default|OnKill _asfirst_person_character)
  (bind _foundwidgets (Widget|GetAllWidgetsOfClass "/Game/UI/PlayerUI.PlayerUI_C" false))
  (Default|ScoreAnim _foundwidgets 1))

(event EventOnDamage
  (params (ProjTransform :type Transform))
  (Audio|SpawnSoundatLocation "/Game/FirstPerson/Audio/HitEnemyLogCue.HitEnemyLogCue" (Transformation|GetWorldLocation (Variables|Default|GetCapsuleComponent)) "0, 0, 0" 1.0 1.0 0.0 0 0)
  (Game|SpawnActorfromClass "/Game/NPC/Enemy/EnemySparks.EnemySparks_C" ProjTransform "Undefined" 0 0)
  (bind _foundwidgets (Widget|GetAllWidgetsOfClass "/Game/UI/PlayerUI.PlayerUI_C" false))
  (Default|ScoreAnim _foundwidgets))

(event EventTick
  (params (DeltaSeconds :type Float%20%28single-precision%29))
  (bind _charactermovement (Variables|Character|GetCharacterMovement))
  (if (Variables|Default|GetSpawnOwnAI)
    (Pawn|SpawnDefaultController)
    (Variables|Default|SetSpawnOwnAI false)
    (else
      (CallFunction|Spin)
      (if (< (Math|Vector|Distance(Vector) (Transformation|GetActorLocation) (Transformation|GetActorLocation (Game|GetPlayerController 0))) (Variables|Default|GetFireRange))
        (CallFunction|Shoot)
        (CallFunction|InView)
        ;[1 1 1] Slow down and stop
        (if (Variables|Default|GetStoppingMovement)
          (if (< (Variables|/Script/Engine.CharacterMovementComponent|GetMaxFlySpeed _charactermovement) 5e+01)
            (Variables|/Script/Engine.CharacterMovementComponent|SetMaxFlySpeed _charactermovement 0.0)
            (else
              (Variables|/Script/Engine.CharacterMovementComponent|SetMaxFlySpeed _charactermovement (- (Variables|/Script/Engine.CharacterMovementComponent|GetMaxFlySpeed _charactermovement) (* (Utilities|Time|GetWorldDeltaSeconds) 3.5e+02))))))))))

(fn ConstructionScript)

(fn Spin
  (Transformation|AddLocalRotation (Variables|Default|GetSpinny) (Math|Rotator|MakeRotator (* (Utilities|Time|GetWorldDeltaSeconds) (Variables|Default|GetSpinSpeed)) 0.0 0.0) false false)
  (Variables|Default|SetSpinSpeed (* (Variables|Default|GetFireTimer) 2e+02)))

(fn Shoot
  (bind _enemymuzzle (Variables|Default|GetEnemyMuzzle))
  (bind _returnvalue (Transformation|GetWorldTransform _enemymuzzle))
  (Variables|Default|SetFireRate (Math|Random|RandomFloatinRange 2.5 3.5))
  (Variables|Default|SetFireTimer (+ (Variables|Default|GetFireTimer) (* (Utilities|Time|GetWorldDeltaSeconds) 1.0)))
  (if (> (Variables|Default|GetFireTimer) (Variables|Default|GetFireRate))
    (Variables|Default|SetFireTimer 0.5)
    (Game|SpawnActorfromClass "/Game/NPC/Enemy/EnemyLaser.EnemyLaser_C" _returnvalue "Undefined" 0 0)
    (Audio|SpawnSoundatLocation "/Game/FirstPerson/Audio/EnemyLasers.EnemyLasers" (.Location (Math|Transform|BreakTransform _returnvalue)) "0, 0, 0" 1.0 1.0 0.0 0 0)))

(fn InView
  (bind _returnvalue (Game|GetPlayerController 0))
  (bind _capsulecomponent (Variables|Default|GetCapsuleComponent))
  (bind (_sizex _sizey) (HUD|GetViewportSize _returnvalue))
  (bind _returnvalue_2 (Transformation|GetWorldLocation _capsulecomponent))
  (bind _screenlocation (Class|PlayerController|ProjectWorldLocationtoScreen _returnvalue _returnvalue_2 false))
  (if (Math|Boolean|ANDBoolean (> (.x _screenlocation) 0.0) (> (.y _screenlocation) 0.0) (< (.x _screenlocation) (Math|Conversions|ToFloat(Integer) _sizex)) (< (.y _screenlocation) (Math|Conversions|ToFloat(Integer) _sizey)))
    (Variables|Default|SetEnemyInView true)
    (else
      (Variables|Default|SetEnemyInView false))))