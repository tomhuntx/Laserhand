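; GameModeHalf_BP, judging by its name a game mode, sets enemy spawn tuning from the selected difficulty.
; On BeginPlay it casts the game instance to Settings_BP and switches on Difficulty02 between Easy, Hard and Impossible, with Easy as the fallback.
; Each tier writes spawn speed rate, boss chance, spawn time range and group chance, with higher tiers generally more punishing.
; The spawning logic that consumes these values lives outside this graph.
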(event EventBeginPlay
  (bind _assettings_bp (Utilities|Casting|CastToSettings_BP (Game|GetGameInstance)))
  (switch int (Variables|/Game/FirstPersonCPP/Blueprints/Settings_BP.Settings_BP_C|GetDifficulty0-2 _assettings_bp)
    (:Default
      ;[1 1 1] Easy
      (Utilities|FlowControl|Sequence :!label _label
        (:then_0
          (Variables|Default|SetSpawnSpeedRate 0.005))
        (:then_1
          (Variables|Default|SetBossChance 0.1))
        (:then_2
          (Variables|Default|SetSpawn_Time_Min 5.0))
        (:then_3
          (Variables|Default|SetSpawn_Time_Max 6.0))
        (:then_4
          (Variables|Default|SetGroupChance 0.15))))
    (:0
      (goto _label))
    (:1
      ;[1 1 1] Hard
      (Utilities|FlowControl|Sequence
        (:then_0
          (Variables|Default|SetSpawnSpeedRate 0.0055))
        (:then_1
          (Variables|Default|SetBossChance 0.15))
        (:then_2
          (Variables|Default|SetSpawn_Time_Min 4.0))
        (:then_3
          (Variables|Default|SetSpawn_Time_Max 5.0))
        (:then_4
          (Variables|Default|SetGroupChance 0.2))))
    (:2
      ;[1 1 1] Impossible
      (Utilities|FlowControl|Sequence
        (:then_0
          (Variables|Default|SetSpawnSpeedRate 0.006))
        (:then_1
          (Variables|Default|SetBossChance 0.25))
        (:then_2
          (Variables|Default|SetSpawn_Time_Min 2.5))
        (:then_3
          (Variables|Default|SetSpawn_Time_Max 3.5))
        (:then_4
          (Variables|Default|SetGroupChance 0.2))))))

(fn ConstructionScript)